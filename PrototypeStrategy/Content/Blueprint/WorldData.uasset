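; WorldData is an actor Blueprint that holds GridData, a map from 2D coordinates to cell records with move cost, path and selection state, apparently for grid movement.
; Its only active logic is DebugPrintData, which walks the map's keys and matching values by index and prints each cell's fields, including path length and accumulated cost.
; BeginPlay, Tick, overlap and the construction script are empty.
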(event `DebugPrintData`
  (bind _griddata (`self.GridData`))
  (bind _keys (`BlueprintMapLibrary.Map_Keys` _griddata))
  (bind _values (`BlueprintMapLibrary.Map_Values` _griddata))
  (for (_array_element _array_index) _keys
    (bind (_movecost _waytopoint _isselect _movecosttothispoint) (break `DataGrid1` (`|GetArrayItem` _values _array_index)))
    (`KismetSystemLibrary.PrintString` (`KismetStringLibrary.Concat_StrStr` "2D Vec: " (`KismetStringLibrary.Conv_Vector2dToString` _array_element) " Index: " (`KismetStringLibrary.Conv_IntToString` _array_index) " MoveCost: " (`KismetStringLibrary.Conv_IntToString` _movecost) " Lenght: " (`KismetStringLibrary.Conv_IntToString` (`KismetArrayLibrary.Array_Length` _waytopoint)) " IsSelect: " (`KismetStringLibrary.Conv_BoolToString` _isselect) " ToCost: " (`KismetStringLibrary.Conv_IntToString` _movecosttothispoint)))))

(fn `UserConstructionScript`)