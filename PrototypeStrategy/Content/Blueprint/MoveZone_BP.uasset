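; Grid map actor that generates a random field of open and blocked cells on BeginPlay and displays a move zone over it.
; BuildZone1 adds open or blocked tile instances, spawns an indexed TitleCollision_BP per cell, and fills the Cells and MapMaskBP arrays.
; BuildMoveZone overlays MoveZone instances on cells with positive Test values, and DeleteMoveZone clears them.
; The unrandomized BuildZone is never run.
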(event `self.ReceiveBeginPlay`
  (set `self.Show` false)
  (`self.BuildZone_1`))

(event `DeleteMoveZone`
  (`InstancedStaticMeshComponent.ClearInstances` (`self.MoveZone`)))

(event `BuildMoveZone`
  (bind (_returnvalue_x _returnvalue_y _returnvalue_z) (`KismetMathLibrary.BreakVector` (`self.K2_GetActorLocation`)))
  (for _index (range (* (`self.SizeX`) (`self.SizeY`)))
    (if (> (`|GetArrayItem` (`self.test`) _index) 0)
      (`InstancedStaticMeshComponent.AddInstance` (`self.MoveZone`) (`KismetMathLibrary.MakeTransform` (- (`KismetMathLibrary.MakeVector` (.x (`.PointVec` (break `DataGrid1` (`|GetArrayItem` (`self.cells`) _index)))) (.y (`.PointVec` (break `DataGrid1` (`|GetArrayItem` (`self.cells`) _index)))) (+ _returnvalue_z 2.5)) (`self.K2_GetActorLocation`)))))))

(fn `BuildZone`
  (bind _sizebeetwencells (`self.SizeBeetwenCells`))
  (bind _sizex (`self.SizeX`))
  (for _index (range (* (`self.SizeX`) (`self.SizeY`)))
    (bind _returnvalue (`KismetMathLibrary.MakeVector` (`KismetMathLibrary.Conv_IntToDouble` (* (/ _index _sizex) _sizebeetwencells)) (`KismetMathLibrary.Conv_IntToDouble` (* (mod _index _sizex) _sizebeetwencells))))
    (`InstancedStaticMeshComponent.AddInstance` (`self.InstancedStaticMesh`) (`KismetMathLibrary.MakeTransform` _returnvalue))
    (bind _returnvalue_2 (+ (`self.K2_GetActorLocation`) _returnvalue))
    (bind _returnvalue_3 (`|SpawnActorFromClass` "/Game/Blueprint/TestPrototypeLevel/TitleCollision_BP.TitleCollision_BP_C" (`KismetMathLibrary.MakeTransform` _returnvalue_2) "Undefined" "OverrideRootScale" null null))
    (`/Game/Blueprint/TestPrototypeLevel/TitleCollision_BP.SetSize` _returnvalue_3 60.0)
    (set `/Game/Blueprint/TestPrototypeLevel/TitleCollision_BP.index` _index _returnvalue_3)
    (`KismetArrayLibrary.Array_Add` (`self.cells`) (make `DataGrid1` :`PointVec` (`KismetMathLibrary.MakeVector` (.x _returnvalue_2) (.y _returnvalue_2))))))

(fn `BuildZone_1`
  (locals (RandomInt :type Integer))
  (bind _sizebeetwencells (`self.SizeBeetwenCells`))
  (bind _sizex (`self.SizeX`))
  (bind _returnvalue (>= (`local.RandomInt`) 2))
  (for _index (range (* (`self.SizeX`) (`self.SizeY`)))
    (bind _output_get (set `local.RandomInt` (`KismetMathLibrary.RandomIntegerInRange` 0 5)))
    (if (>= _output_get 2)
      (bind _returnvalue_2 (`KismetMathLibrary.MakeVector` (`KismetMathLibrary.Conv_IntToDouble` (* (/ _index _sizex) _sizebeetwencells)) (`KismetMathLibrary.Conv_IntToDouble` (* (mod _index _sizex) _sizebeetwencells))))
      (bind _returnvalue_3 (`KismetMathLibrary.MakeTransform` _returnvalue_2))
      (`InstancedStaticMeshComponent.AddInstance` (`self.InstancedStaticMesh`) _returnvalue_3)
      (else
        (`InstancedStaticMeshComponent.AddInstance` (`self.BlockZone`) _returnvalue_3)))
    (bind _returnvalue_4 (+ (`self.K2_GetActorLocation`) _returnvalue_2))
    (bind _returnvalue_5 (`|SpawnActorFromClass` "/Game/Blueprint/TestPrototypeLevel/TitleCollision_BP.TitleCollision_BP_C" (`KismetMathLibrary.MakeTransform` _returnvalue_4) "Undefined" "OverrideRootScale" null null))
    (`/Game/Blueprint/TestPrototypeLevel/TitleCollision_BP.SetSize` _returnvalue_5 60.0)
    (set `/Game/Blueprint/TestPrototypeLevel/TitleCollision_BP.index` _index _returnvalue_5)
    (`KismetArrayLibrary.Array_Add` (`self.cells`) (make `DataGrid1` :`isSelect` (not _returnvalue) :`PointVec` (`KismetMathLibrary.MakeVector` (.x _returnvalue_4) (.y _returnvalue_4))))
    (`KismetArrayLibrary.Array_Add` (`self.mapMask_BP`) (select `bool` _returnvalue :`false` 1 :`true` 0))))

(fn `ClearArray`
  (bind _cells (`self.cells`))
  (for (_array_element _array_index) _cells
    (bind (_movecost _waytopoint _isselect _movecosttothispoint _pointvec) (break `DataGrid1` _array_element))
    (`KismetArrayLibrary.Array_Set` _cells _array_index (make `DataGrid1` :`MoveCost` _movecost :`isSelect` _isselect :`MoveCostToThisPoint` _movecosttothispoint :`PointVec` _pointvec))))

(fn `UserConstructionScript`)