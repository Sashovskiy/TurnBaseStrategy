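; Clickable tile actor with a resizable flat box collider and a text label, used as a move destination with a path and cost.
; SetWay stores the path and appends the tile's location, while event 123456 sets and displays the cost.
; Clicking the box passes the tile's Index to PC_BP's MoveToPoint.
; ClearWay empties the path, zeroes the cost, hides the box and resets the label.
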(event `123456`
  (params (Value :type Integer))
  (set `self.CostTo` Value)
  (`TextRenderComponent.K2_SetText` (`self.TextRender`) (`KismetTextLibrary.Conv_IntToText` Value)))

(event `SetSize`
  (params (`In Box Extent X` :type "Float (double-precision)"))
  (`BoxComponent.SetBoxExtent` (`self.Box`) (`KismetMathLibrary.MakeVector` `In Box Extent X` `In Box Extent X` 5.0) true))

(event `self.ReceiveTick`
  (params (DeltaSeconds :type "Float (single-precision)")))

(event `self.Box.OnBeginCursorOver`
  (params (TouchedComponent :type "PrimitiveComponent Object Reference")))

(event `ClearWay`
  (`KismetArrayLibrary.Array_Clear` (`self.WayToPoint`))
  (set `self.CostTo` 0)
  (`SceneComponent.SetHiddenInGame` (`self.Box`) true false)
  (`TextRenderComponent.K2_SetText` (`self.TextRender`) (`self.DeleteThis`)))

(event `self.Box.OnClicked`
  (params (TouchedComponent :type "PrimitiveComponent Object Reference") (ButtonPressed :type "Key Structure"))
  (bind _aspc_bp (cast `/Game/Blueprint/PC_BP` (`GameplayStatics.GetPlayerController` 0)))
  (`/Game/Blueprint/PC_BP.MoveToPoint` _aspc_bp (`self.index`)))

(fn `SetWay`
  (params (WayToPoint :type "Array of Vector Structure"))
  (bind _output_get (set `self.WayToPoint` WayToPoint))
  (`KismetArrayLibrary.Array_Add` _output_get (`self.K2_GetActorLocation`)))

(fn `UserConstructionScript`)