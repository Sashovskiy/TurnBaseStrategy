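; MainMenu_PC_BP, apparently the main menu player controller, puts the SetData widget on screen at BeginPlay.
; Its SetGrafic event writes a given texture quality level to GameUserSettings, saves it without an explicit apply call, and prints the value.
; An unconnected chain that would create, store and show the MainMenu_w widget never runs.
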(event `self.ReceiveBeginPlay`
  (bind _returnvalue (`|CreateWidget` "/Game/Blueprint/MainMenu_fl/SetData.SetData_C"))
  (`UserWidget.AddToViewport` _returnvalue 0))

(event `SetGrafic`
  (params (Num :type Integer))
  (bind _returnvalue (`GameUserSettings.GetGameUserSettings`))
  (`GameUserSettings.SetTextureQuality` _returnvalue Num)
  (`GameUserSettings.SaveSettings` _returnvalue)
  (`KismetSystemLibrary.PrintString` (`KismetStringLibrary.Conv_IntToString` (`GameUserSettings.GetTextureQuality` _returnvalue))))

(fn `UserConstructionScript`)