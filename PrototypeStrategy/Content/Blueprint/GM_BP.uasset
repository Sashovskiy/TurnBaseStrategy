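; Game mode Blueprint that sets up the level on BeginPlay from grid settings stored in the game instance.
; It spawns the MoveZone grid, places the character on the first cell not flagged IsSelect, and spawns WorldData.
; It then initializes the player controller and, after a short delay, moves the camera to the main character.
; A validity macro prints Yes or No after key steps and halts the chain on failure.
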(event `self.ReceiveBeginPlay`
  (bind _inc (`self.Inc`))
  (bind _asmy_game_inst (cast `/Game/Blueprint/MyGameInst` (`GameplayStatics.GetGameInstance`)))
  (`self.NewMacro_0` _asmy_game_inst)
  (bind (_sizex _sizey _sizebeetwen) (`/Game/Blueprint/MyGameInst.GetMoveZoneData` _asmy_game_inst))
  (`self.SetMoveZoneData` _sizex _sizey _sizebeetwen)
  (bind _returnvalue (`|SpawnActorFromClass` "/Game/Blueprint/MoveZone_BP.MoveZone_BP_C" (`KismetMathLibrary.MakeTransform` (1390.0 1440.0 20.0)) "Undefined" "OverrideRootScale" null null))
  (`self.NewMacro_0` _returnvalue)
  (`MoveZone.SetMoveZoneData` _returnvalue (`self.SizeX`) (`self.SizeY`) (`self.SizeBeetwen`))
  (bind ((`isSelect` _isselect) (`PointVec` _pointvec)) (break `DataGrid1` (`|GetArrayItem` (`MoveZone.cells` _returnvalue) _inc)))
  (while _isselect
    (`/Engine/EditorBlueprintResources/StandardMacros.IncrementInt` _inc))
  (bind _returnvalue_2 (`|SpawnActorFromClass` "/Game/Blueprint/ParentCharecter_BP.ParentCharecter_BP_C" (`KismetMathLibrary.MakeTransform` (`KismetMathLibrary.MakeVector` (.x _pointvec) (.y _pointvec) 108.0)) "AlwaysSpawn" "OverrideRootScale" null null))
  (`self.NewMacro_0` _returnvalue_2)
  (bind _returnvalue_3 (`|SpawnActorFromClass` "/Game/Blueprint/WorldData.WorldData_C" (`KismetMathLibrary.MakeTransform` (0.0 0.0 0.0)) "Undefined" "OverrideRootScale" null null))
  (`self.NewMacro_0` _returnvalue_3)
  (bind _aspc_bp (cast `/Game/Blueprint/PC_BP` (`GameplayStatics.GetPlayerController` 0)))
  (`self.NewMacro_0` _aspc_bp)
  (`/Game/Blueprint/PC_BP.BeginP` _aspc_bp)
  (`KismetSystemLibrary.Delay` 2.0)
  (`/Game/Blueprint/PC_BP.CameraToMainChar` _aspc_bp))

(fn `SetMoveZoneData`
  (params (SizeX :type Integer) (SizeY :type Integer) (SizeBeetwen :type Integer))
  (set `self.SizeX` SizeX)
  (set `self.SizeY` SizeY)
  (set `self.SizeBeetwen` SizeBeetwen))

(fn `UserConstructionScript`)